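; Cat action that performs an area-of-effect attack around the owning Cat.
; Its Trigger override calls the parent, runs a sphere overlap-style trace at the Cat's location, then plays a sped-up attack montage.
; Each newly hit actor takes damage credited to the first player controller and receives a damage message if Damageable.
; HittedActors is never cleared here, so previously hit actors are skipped on later triggers.
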(fn `Trigger`
  (params (Owner :type "Character Object Reference"))
  (locals (`Object Types` :type "Array of EObjectTypeQuery Enum") (HittedActors :type "Set of Actor Object Reference"))
  (bind _hittedactors (`local.HittedActors`))
  (`parent.Trigger` Owner)
  (bind _ascat (cast `/Game/Cats/Blueprint/Cat` Owner))
  (bind _returnvalue_location (`KismetMathLibrary.BreakTransform` (`Actor.GetTransform` _ascat)))
  (bind _outhits (`KismetSystemLibrary.SphereTraceMultiForObjects` _returnvalue_location _returnvalue_location 100.0 (`local.Object Types`) false (`|MakeArray` _ascat :!type "Actor Object Reference")))
  (for _array_element _outhits
    (bind (_bblockinghit _binitialoverlap _time _distance _location _impactpoint _normal _impactnormal _physmat _hitactor) (`GameplayStatics.BreakHitResult` _array_element))
    (if (not (`BlueprintSetLibrary.Set_Contains` _hittedactors _hitactor))
      (`BlueprintSetLibrary.Set_Add` _hittedactors _hitactor)
      (`GameplayStatics.ApplyDamage` _hitactor 2.0 (`GameplayStatics.GetPlayerController` 0) _ascat "/Script/Engine.DamageType")
      (if (`KismetSystemLibrary.DoesImplementInterface` _hitactor "/Game/Cats/Blueprint/Interfaces/damageable.damageable_C")
        (message `/Game/Cats/Blueprint/Interfaces/damageable.On Damage` _hitactor (`Actor.K2_GetActorLocation` _hitactor)))))
  (`Character.PlayAnimMontage` _ascat "/Game/Cats/Assets/Cat/Custom/AttackMontage.AttackMontage" 3.0 "None"))