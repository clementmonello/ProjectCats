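; Interactable egg prop that gets knocked away from the player when interacted with.
; OnInteract applies an impulse to the Egg component along the player character's forward vector, scaled by ForceFactor.
; The impulse is applied as a velocity change, so the egg's mass does not affect the launch speed.
; BeginPlay, overlap and Tick are disabled stubs, and the construction script only calls its parent.
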(event `/Game/Cats/Blueprint/Interfaces/interactable.On Interact`
  (bind _returnvalue (`GameplayStatics.GetPlayerCharacter` 0))
  (bind _returnvalue_2 (`self.K2_GetActorLocation` _returnvalue))
  (`PrimitiveComponent.AddImpulse` (`self.Egg`) (* (`KismetMathLibrary.GetDirectionUnitVector` _returnvalue_2 (+ _returnvalue_2 (`self.GetActorForwardVector` _returnvalue))) (`self.ForceFactor`)) "None" true))

(fn `UserConstructionScript`
  (`parent.UserConstructionScript`))