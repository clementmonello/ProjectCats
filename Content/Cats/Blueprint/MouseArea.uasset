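; Mouse hunting zone that offers the cat a "Hunt Mice" mission, shown as a widget while the cat is inside the trigger.
; It registers itself with its listed mice, spawning one if none exist, and tracks the living count via DecreaseMouseAlive.
; Clearing all mice plays an effect, awards nice karma and removes the widget.
; AddNewMouse rejection-samples the spline's bounds with a ray-casting point-in-polygon test to place mice inside the outline.
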(event `self.ReceiveBeginPlay`
  (`KismetSystemLibrary.ExecuteConsoleCommand` "show splines" null)
  (if (`KismetArrayLibrary.Array_IsEmpty` (`self.ListeMouse`))
    (bind _returnvalue (`|SpawnActorFromClass` "/Game/Cats/Blueprint/Mouse.Mouse_C" (`self.GetTransform` self) "AdjustIfPossibleButAlwaysSpawn" "MultiplyWithRoot" null null))
    (`KismetArrayLibrary.Array_Add` (`self.ListeMouse`) _returnvalue))
  (`self.ResetMouseAreaToMouses`))

(event `NoMoreMouse`
  (bind _widgetmission (`self.WidgetMission`))
  (`NiagaraFunctionLibrary.SpawnSystemAtLocation` "/Game/Cats/Assets/Points/bad_200_fx_System.bad_200_fx_System" (+ (`self.K2_GetActorLocation`) (0.0 0.0 10.0)))
  (`/Game/Cats/Blueprint/MainLibrary.AddNiceKarma` 200)
  (set `self.MissionDone` true)
  (`/Engine/EditorBlueprintResources/StandardMacros.IsValid` (`self.WidgetMission`) :!label _label
    (:`Is Valid`
      (`UserWidget.PlayAnimation` _widgetmission (`/Game/Cats/Widget/GoodMissionMenu.NewMission` _widgetmission) 0.0 1 "Reverse" 1.0 false)
      (`KismetSystemLibrary.Delay` 0.3)
      (`Widget.RemoveFromParent` _widgetmission))))

(event `self.Entering Area.OnComponentEndOverlap`
  (params (OverlappedComponent :type "PrimitiveComponent Object Reference") (OtherActor :type "Actor Object Reference") (OtherComp :type "PrimitiveComponent Object Reference") (OtherBodyIndex :type Integer))
  (if (not (`self.MissionDone`))
    (cast `/Game/Cats/Blueprint/Cat` OtherActor)
    (goto _label)))

(event `self.Entering Area.OnComponentBeginOverlap`
  (params (OverlappedComponent :type "PrimitiveComponent Object Reference") (OtherActor :type "Actor Object Reference") (OtherComp :type "PrimitiveComponent Object Reference") (OtherBodyIndex :type Integer) (bFromSweep :type Boolean) (SweepResult :type "HitResult Structure (by ref)"))
  (if (not (`self.MissionDone`))
    (cast `/Game/Cats/Blueprint/Cat` OtherActor)
    (bind _returnvalue (`|CreateWidget` "/Game/Cats/Widget/GoodMissionMenu.GoodMissionMenu_C" (`GameplayStatics.GetPlayerController` 0)))
    (set `/Game/Cats/Widget/GoodMissionMenu.GoodMissionText` "Hunt Mice" _returnvalue)
    (bind _output_get (set `self.WidgetMission` _returnvalue))
    (`UserWidget.AddToViewport` _output_get 0)
    (`UserWidget.PlayAnimation` _output_get (`/Game/Cats/Widget/GoodMissionMenu.NewMission` _output_get) 0.1 1 "Forward" 1.0 false)))

(fn `AddNewMouse`
  (locals (pointTested :type "Vector Structure" :default (0.0 0.0 0.0)))
  (bind (_origin _boxextent) (`KismetSystemLibrary.GetComponentBounds` (`self.Spline`)))
  (bind _polygon (`self.GetPolygon`))
  (set `self.Polygon` _polygon)
  (bind _output_get (set `local.pointTested` (`KismetMathLibrary.RandomPointInBoundingBox` _origin _boxextent) :!label _label))
  (bind _isinside (`self.IsPointInPolygon` _output_get (`self.Polygon`)))
  (if _isinside
    (bind _returnvalue (`|SpawnActorFromClass` "/Game/Cats/Blueprint/Mouse.Mouse_C" (`KismetMathLibrary.Conv_VectorToTransform` (`local.pointTested`)) "AdjustIfPossibleButAlwaysSpawn" "MultiplyWithRoot" null null))
    (`KismetArrayLibrary.Array_Add` (`self.ListeMouse`) _returnvalue)
    (else
      (goto _label))))

(fn `DecreaseMouseAlive`
  (bind _output_get (set `self.NbMouseAlive` (- (`self.NbMouseAlive`) 1)))
  (`KismetSystemLibrary.PrintString` (`KismetStringLibrary.Conv_IntToString` _output_get))
  (if (== _output_get 0)
    (`self.NoMoreMouse`)))

(fn `GetPolygon`
  (returns (Polygon :type "Array of Vector Structure"))
  (locals (Corner :type "Array of Vector Structure"))
  (for _index (range (`SplineComponent.GetNumberOfSplinePoints` (`self.Spline`)))
    (`KismetArrayLibrary.Array_Add` (`local.Corner`) (`SplineComponent.GetLocationAtSplinePoint` (`self.Spline`) _index "World")))
  (return (`local.Corner`)))

(fn `IsPointInPolygon`
  (params (Point :type "Vector Structure") (Polygon :type "Array of Vector Structure"))
  (returns (isInside :type Boolean))
  (locals (NumPoints :type Integer) (Return :type Boolean) (indexi :type Integer) (indexj :type Integer))
  (bind _numpoints (`local.NumPoints`))
  (bind (_point_x _point_y) (`KismetMathLibrary.BreakVector` (`local.Point`)))
  (bind (_point_x_2 _point_y_2) (`KismetMathLibrary.BreakVector` (`local.Point`)))
  (bind (_point_x_3 _point_y_3) (`KismetMathLibrary.BreakVector` (`local.Point`)))
  (bind (_output_x _output_y) (`KismetMathLibrary.BreakVector` (`|GetArrayItem` (`local.Polygon`) (`local.indexi`))))
  (bind _output_x_2 (`KismetMathLibrary.BreakVector` (`|GetArrayItem` (`local.Polygon`) (`local.indexi`))))
  (bind (_output_x_3 _output_y_2) (`KismetMathLibrary.BreakVector` (`|GetArrayItem` (`local.Polygon`) (`local.indexi`))))
  (bind (_output_x_4 _output_y_3) (`KismetMathLibrary.BreakVector` (`|GetArrayItem` (`local.Polygon`) (`local.indexj`))))
  (bind (_output_x_5 _output_y_4) (`KismetMathLibrary.BreakVector` (`|GetArrayItem` (`local.Polygon`) (`local.indexj`))))
  (bind _output_x_6 (`KismetMathLibrary.BreakVector` (`|GetArrayItem` (`local.Polygon`) (`local.indexj`))))
  (set `local.NumPoints` (`KismetArrayLibrary.Array_Length` Polygon))
  (set `local.Return` false)
  (for _index (range (`local.NumPoints`))
    (bind _output_get (set `local.indexi` _index))
    (set `local.indexj` (mod (+ _output_get _numpoints -1) _numpoints))
    (if (and (!= (> _output_y_2 _point_y_3) (> _output_y_3 _point_y)) (< _point_x_2 (+ (* (- _output_x_6 _output_x_2) (/ (- _point_y_2 _output_y) (- _output_y_4 _output_y))) _output_x)))
      (set `local.Return` (not (`local.Return`)))))
  (return (`local.Return`)))

(fn `ResetMouseAreaToMouses`
  (for _array_element (`self.ListeMouse`)
    (set `/Game/Cats/Blueprint/Mouse.MouseArea` self _array_element)
    (set `self.NbMouseAlive` (+ (`self.NbMouseAlive`) 1))))

(fn `UserConstructionScript`)