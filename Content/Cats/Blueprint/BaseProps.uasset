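; BaseProps is the base Blueprint for damageable props in a cat game, adding bad karma when they are damaged.
; Each OnDamage call spawns a CatStrainField actor at the supplied location, regardless of collision.
; A CanGivePoint flag limits the karma gain and a Niagara effect, spawned slightly above that location, to the first hit that finds it set.
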(event `self.ReceiveBeginPlay`)

(event `/Game/Cats/Blueprint/Interfaces/damageable.On Damage`
  (params (Localisation :type "Vector Structure"))
  (`|SpawnActorFromClass` "/Game/Cats/Blueprint/CatStrainField.CatStrainField_C" (`KismetMathLibrary.MakeTransform` Localisation) "AlwaysSpawn" "MultiplyWithRoot" null null)
  (if (`self.CanGivePoint`)
    (set `self.CanGivePoint` false)
    (`/Game/Cats/Blueprint/MainLibrary.AddBadKarma` 25)
    (`NiagaraFunctionLibrary.SpawnSystemAtLocation` (`self.System Template`) (+ Localisation (0.0 0.0 50.0)) (struct) (0.8 0.8 0.8))))

(fn `UserConstructionScript`)