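; Area-of-effect attack action component for cats, damaging actors around the owner when triggered.
; Trigger calls the parent, then runs a multi-sphere object trace at the owning Cat's location, scaling the radius by its range multiplier.
; Each hit actor not already in HittedActors receives fixed damage and, if Damageable, a damage message; the list is never cleared here.
; The trace's debug drawing is left enabled.
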(fn `Trigger`
  (params (Owner :type "Character Object Reference"))
  (bind _hittedactors (`self.HittedActors`))
  (bind _returnvalue_location (`KismetMathLibrary.BreakTransform` (`Actor.GetTransform` (`local.Owner`))))
  (`parent.Trigger` Owner)
  (bind _ascat (cast `/Game/Cats/Blueprint/Cat` Owner))
  (bind _outhits (`KismetSystemLibrary.SphereTraceMultiForObjects` :`Start` _returnvalue_location :`End` _returnvalue_location :`Radius` (* (`self.Radius`) (`/Game/Cats/Blueprint/Cat.RangeMultiplicator` _ascat)) :`ObjectTypes` (`self.Object Types`) :`DrawDebugType` "ForDuration"))
  (for _array_element _outhits
    (bind (_bblockinghit _binitialoverlap _time _distance _location _impactpoint _normal _impactnormal _physmat _hitactor) (`GameplayStatics.BreakHitResult` _array_element))
    (if (not (`BlueprintSetLibrary.Set_Contains` _hittedactors _hitactor))
      (`BlueprintSetLibrary.Set_Add` _hittedactors _hitactor)
      (`GameplayStatics.ApplyDamage` _hitactor 2.0 null (`local.Owner`) "/Script/Engine.DamageType")
      (if (`KismetSystemLibrary.DoesImplementInterface` _hitactor "/Game/Cats/Blueprint/Interfaces/damageable.damageable_C")
        (message `/Game/Cats/Blueprint/Interfaces/damageable.On Damage` _hitactor (`Actor.K2_GetActorLocation` _hitactor))))))