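; Attack action component for cats that damages objects in front of the triggering cat.
; When triggered, it casts the owner to Cat and runs a forward multi-object box trace, with reach and box size scaled by the cat's range multiplier.
; Each hit receives fixed damage, and actors implementing Damageable also get a damage message with the impact point.
; The trace has debug drawing enabled.
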(fn `Trigger`
  (params (Owner :type "Character Object Reference"))
  (bind _cat (`self.Cat`))
  (bind _rangemultiplicator (`/Game/Cats/Blueprint/Cat.RangeMultiplicator` _cat))
  (bind _returnvalue (+ (`Actor.K2_GetActorLocation` _cat) (`/Game/Cats/Blueprint/Cat.CapsuleHeightAdjust` _cat)))
  (`parent.Trigger` Owner)
  (bind _ascat (cast `/Game/Cats/Blueprint/Cat` Owner))
  (set `self.Cat` _ascat)
  (bind (_outhits _returnvalue_2) (`KismetSystemLibrary.BoxTraceMultiForObjects` :`Start` _returnvalue :`End` (+ _returnvalue (* (`Actor.GetActorForwardVector` _cat) (`/Game/Cats/Blueprint/Cat.CapsuleInteractDistance` _cat) _rangemultiplicator)) :`HalfSize` (* (`self.HalfSize`) _rangemultiplicator) :`ObjectTypes` (`self.Object Types`) :`DrawDebugType` "ForDuration"))
  (if _returnvalue_2
    (for _array_element _outhits
      (bind (_bblockinghit _binitialoverlap _time _distance _location _impactpoint _normal _impactnormal _physmat _hitactor) (`GameplayStatics.BreakHitResult` _array_element))
      (`GameplayStatics.ApplyDamage` _hitactor 1.0 (`GameplayStatics.GetPlayerController` 0) (`self.Cat`) "/Script/Engine.DamageType")
      (if (`KismetSystemLibrary.DoesImplementInterface` _hitactor "/Game/Cats/Blueprint/Interfaces/damageable.damageable_C")
        (message `/Game/Cats/Blueprint/Interfaces/damageable.On Damage` _hitactor _impactpoint)))))