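; C_ACT_Range is a cat component that scales the range stat of the Cat it is attached to.
; On BeginPlay it calls GiveStats, which casts the owner to Cat and multiplies its RangeMultiplicator by the component's RangeAmount.
; The change stacks multiplicatively with the existing value, and nothing in the component reverts it.
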(event `self.ReceiveBeginPlay`
  (`parent.ReceiveBeginPlay`)
  (`self.giveStats`))

(fn `giveStats`
  (bind _ascat (cast `/Game/Cats/Blueprint/Cat` (`self.GetOwner` self)))
  (set `/Game/Cats/Blueprint/Cat.RangeMultiplicator` (* (`/Game/Cats/Blueprint/Cat.RangeMultiplicator` _ascat) (`self.rangeAmount`)) _ascat))