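; Actor component that steers its owner along a BP_TargetSpline, optionally picking the one nearest its forward aim point on BeginPlay.
; Each tick it records spline progress and takes the closest spline point to that look-ahead point as destination, read in Local space but used as world.
; Pawns receive movement input toward it, while other actors move along local forward and rotate to face it.
; Optional debug spheres show both points.
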(event `self.ReceiveBeginPlay`
  (if (`self.AutoFindSpline`)
    (bind _outactors (`GameplayStatics.GetAllActorsOfClass` "/Game/Cats/Blueprint/BP_TargetSpline.BP_TargetSpline_C"))
    (bind _asbp_target_spline (cast `/Game/Cats/Blueprint/BP_TargetSpline` (`.ReturnValue` (`GameplayStatics.FindNearestActor` (`self.GetForwardAimLocation`) _outactors))))
    (set `self.Target Spline` _asbp_target_spline)))

(event `self.ReceiveTick`
  (params (DeltaSeconds :type "Float (single-precision)"))
  (`self.GetCurrentDistaneOnSpline`)
  (`self.UpdateDestination`)
  (`self.ProceedToDestination` DeltaSeconds)
  (if (`self.DrawDebug`)
    (`self.UpdateDebug`)))

(fn `GetCurrentDistaneOnSpline`
  (returns (PercentageAlongSpline :type "Float (double-precision)"))
  (bind _spline (`/Game/Cats/Blueprint/BP_TargetSpline.Spline` (`self.Target Spline`)))
  (bind _output_get (set `self.DistanceAlongSpline` (`SplineComponent.GetDistanceAlongSplineAtSplineInputKey` _spline (`SplineComponent.FindInputKeyClosestToWorldLocation` _spline (`Actor.K2_GetActorLocation` (`self.GetOwner`))))))
  (bind _output_get_2 (set `self.PercentageAlongSpline` (* (/ _output_get (`SplineComponent.GetSplineLength` _spline)) 100.0)))
  (return _output_get_2))

(fn `GetForwardAimLocation`
  (returns (FrontLocation :type "Vector Structure"))
  (bind _returnvalue (`self.GetOwner`))
  (return (+ (`Actor.K2_GetActorLocation` _returnvalue) (* (`Actor.GetActorForwardVector` _returnvalue) (`self.ForwardAimDistance`)))))

(fn `ProceedToDestination`
  (params (DeltaTime :type "Float (double-precision)"))
  (locals (TimeSinceLastUpdate :type "Float (double-precision)"))
  (bind _returnvalue (`self.GetOwner`))
  (bind _returnvalue_2 (`self.GetOwner`))
  (bind _rootcomponent (`Actor.RootComponent` _returnvalue))
  (set `local.TimeSinceLastUpdate` DeltaTime)
  ;[1 1 1] Pawn/Character Movement
  (bind _aspawn (cast `Pawn` _returnvalue_2)
    (:`then`
      (`Pawn.AddMovementInput` _aspawn (`KismetMathLibrary.GetForwardVector` (`KismetMathLibrary.FindLookAtRotation` (`SceneComponent.K2_GetComponentLocation` (`Actor.RootComponent` _returnvalue_2)) (`self.Destination`))) (`self.Speed`) true))
    (:`CastFailed`
      ;[1 1 1] Movement for basic objects
      (`Actor.K2_AddActorLocalOffset` _returnvalue (`KismetMathLibrary.MakeVector` (* (`self.Speed`) (`self.MaxSpeed (cm/s)`) (`local.TimeSinceLastUpdate`))) false false)
      (`SceneComponent.K2_SetWorldRotation` _rootcomponent (`KismetMathLibrary.FindLookAtRotation` (`SceneComponent.K2_GetComponentLocation` _rootcomponent) (`self.Destination`)) false false))))

(fn `UpdateDebug`
  (`KismetSystemLibrary.DrawDebugSphere` (`self.Destination`) 10.0 12 (struct :`R` 1.0 :`G` 0.130541 :`B` 0.070812 :`A` 1.0))
  (`KismetSystemLibrary.DrawDebugSphere` (`self.GetForwardAimLocation`)))

(fn `UpdateDestination`
  (returns (Destination :type "Vector Structure"))
  (bind _output_get (set `self.Destination` (`SplineComponent.FindLocationClosestToWorldLocation` (`/Game/Cats/Blueprint/BP_TargetSpline.Spline` (`self.Target Spline`)) (`self.GetForwardAimLocation`) "Local")))
  (return _output_get))