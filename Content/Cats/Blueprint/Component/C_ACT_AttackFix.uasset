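; Cat action component that repairs props in front of the cat when triggered, by calling Regen on them.
; Trigger runs the parent logic, then casts the owner to Cat and box-traces forward from its height-adjusted location.
; The cat's range multiplier scales both trace distance and box size.
; Every BaseProps actor hit gets Regen, and the trace draws debug shapes for a duration.
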(fn `Trigger`
  (params (Owner :type "Character Object Reference"))
  (bind _as_cat (`self.As Cat`))
  (bind _rangemultiplicator (`/Game/Cats/Blueprint/Cat.RangeMultiplicator` _as_cat))
  (bind _returnvalue (+ (`Actor.K2_GetActorLocation` _as_cat) (`/Game/Cats/Blueprint/Cat.CapsuleHeightAdjust` _as_cat)))
  (`parent.Trigger` Owner)
  (bind _ascat (cast `/Game/Cats/Blueprint/Cat` Owner))
  (set `self.As Cat` _ascat)
  (bind (_outhits _returnvalue_2) (`KismetSystemLibrary.BoxTraceMultiForObjects` :`Start` _returnvalue :`End` (+ _returnvalue (* (`Actor.GetActorForwardVector` _as_cat) (`/Game/Cats/Blueprint/Cat.CapsuleInteractDistance` _as_cat) _rangemultiplicator)) :`HalfSize` (* (`self.HalfSize`) _rangemultiplicator) :`ObjectTypes` (`self.Object Types`) :`DrawDebugType` "ForDuration"))
  (if _returnvalue_2
    (for _array_element _outhits
      (bind _asbase_props (cast `/Game/Cats/Blueprint/BreakableProps/BaseProps` (`.HitActor` (`GameplayStatics.BreakHitResult` _array_element))))
      (`/Game/Cats/Blueprint/BreakableProps/BaseProps.Regen` _asbase_props))))