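; Cat ability component, "Corrupted Miaou", that replaces nearby mice with summoned ones when triggered.
; Trigger calls the parent, then runs a multi-sphere object trace at the Cat, with Range scaled by its RangeMultiplicator and debug drawing enabled.
; Each Mouse hit is destroyed after a SumonedMouse spawns at its transform.
; A Niagara effect, also scaled by the range multiplier, then plays at the owner.
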(fn `Trigger`
  (params (Owner :type "Character Object Reference"))
  (bind (_returnvalue_location _returnvalue_rotation) (`KismetMathLibrary.BreakTransform` (`Actor.GetTransform` (`self.GetOwner`))))
  (`parent.Trigger` Owner)
  (bind _ascat (cast `/Game/Cats/Blueprint/Cat` Owner))
  (bind _returnvalue_location_2 (`KismetMathLibrary.BreakTransform` (`Actor.GetTransform` _ascat)))
  (bind _outhits (`KismetSystemLibrary.SphereTraceMultiForObjects` :`Start` _returnvalue_location_2 :`End` _returnvalue_location_2 :`Radius` (* (`self.Range`) (`/Game/Cats/Blueprint/Cat.RangeMultiplicator` _ascat)) :`ObjectTypes` (`self.Object Types`) :`DrawDebugType` "ForDuration"))
  (for _array_element _outhits
    (bind _asmouse (cast `/Game/Cats/Blueprint/Mouse` (`.HitActor` (`GameplayStatics.BreakHitResult` _array_element))))
    (`|SpawnActorFromClass` "/Game/Cats/Blueprint/SumonedMouse.SumonedMouse_C" (`Actor.GetTransform` _asmouse) "AlwaysSpawn" "MultiplyWithRoot" null null)
    (`Actor.K2_DestroyActor` _asmouse))
  (`NiagaraFunctionLibrary.SpawnSystemAtLocation` (`self.Particle`) _returnvalue_location _returnvalue_rotation (`KismetMathLibrary.Conv_DoubleToVector` (* (`/Game/Cats/Blueprint/Cat.RangeMultiplicator` _ascat) 3.0))))