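; Base Blueprint for breakable props that shatter when damaged and award bad karma once.
; OnDamage hides the physics-simulated static mesh, moves the Chaos GeometryCollection to its transform, enables physics and spawns a field actor at the hit location to break it.
; The first break also spawns a particle effect.
; Regen replaces a broken prop by spawning a new instance of its class at the collection's location with an effect, then destroying itself.
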(event `self.ReceiveBeginPlay`
  (`SceneComponent.SetHiddenInGame` (`self.GeometryCollection`) false false)
  (`PrimitiveComponent.SetSimulatePhysics` (`self.StaticMesh1`) true))

(event `/Game/Cats/Blueprint/Interfaces/damageable.On Damage`
  (params (Localisation :type "Vector Structure"))
  (bind _geometrycollection (`self.GeometryCollection`))
  (bind _staticmesh1 (`self.StaticMesh1`))
  (if (not (`SceneComponent.bHiddenInGame` _staticmesh1))
    (`SceneComponent.SetHiddenInGame` _staticmesh1 true false)
    (`SceneComponent.K2_SetWorldTransform` _geometrycollection (`SceneComponent.K2_GetComponentToWorld` _staticmesh1) false true)
    (`SceneComponent.SetHiddenInGame` _geometrycollection false false)
    (set `GeometryCollectionComponent.ObjectType` "Chaos_Object_Dynamic" _geometrycollection)
    (`|SpawnActorFromClass` "/Game/Cats/Blueprint/FS_MasterField_2.FS_MasterField_2_C" (`KismetMathLibrary.MakeTransform` Localisation (struct) (1.3 1.3 1.3)) "AlwaysSpawn" "MultiplyWithRoot" null null)
    (`PrimitiveComponent.SetSimulatePhysics` _geometrycollection true)
    (`PrimitiveComponent.SetEnableGravity` _geometrycollection true)
    (if (`self.CanGivePoint`)
      (set `self.CanGivePoint` false)
      (`/Game/Cats/Blueprint/MainLibrary.AddBadKarma` 25)
      (`NiagaraFunctionLibrary.SpawnSystemAtLocation` (`self.System Template`) (+ Localisation (0.0 0.0 50.0)) (struct) (0.8 0.8 0.8)))))

(fn `Regen`
  (bind _returnvalue (`SceneComponent.K2_GetComponentLocation` (`self.GeometryCollection`)))
  (if (not (`self.CanGivePoint`))
    (`|SpawnActorFromClass` (`GameplayStatics.GetObjectClass` self) (`KismetMathLibrary.MakeTransform` _returnvalue) "AdjustIfPossibleButAlwaysSpawn" "MultiplyWithRoot" null null)
    (`NiagaraFunctionLibrary.SpawnSystemAtLocation` "/Game/Cats/Assets/Niagara/NS_Cat_16.NS_Cat_16" _returnvalue (struct) (1.5 1.5 1.5))
    (`self.K2_DestroyActor`)))

(fn `UserConstructionScript`)