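; Breakable egg prop that the player can knock around and smash to earn bad karma.
; Interacting launches the Egg component along the player character's forward vector, using a velocity-change impulse scaled by ForceFactor.
; Each damage event spawns a CatStrainField at the given location, presumably to fracture the egg.
; The first hit also adds bad karma and shows a floating effect, gated by CanGivePoint.
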(event `/Game/Cats/Blueprint/Interfaces/interactable.On Interact`
  (bind _returnvalue (`GameplayStatics.GetPlayerCharacter` 0))
  (bind _returnvalue_2 (`self.K2_GetActorLocation` _returnvalue))
  (`PrimitiveComponent.AddImpulse` (`self.Egg`) (* (`KismetMathLibrary.GetDirectionUnitVector` _returnvalue_2 (+ _returnvalue_2 (`self.GetActorForwardVector` _returnvalue))) (`self.ForceFactor`)) "None" true))

(event `/Game/Cats/Blueprint/Interfaces/damageable.On Damage`
  (params (Localisation :type "Vector Structure"))
  (`|SpawnActorFromClass` "/Game/Cats/Blueprint/CatStrainField.CatStrainField_C" (`KismetMathLibrary.MakeTransform` Localisation) "Undefined" "MultiplyWithRoot" null null)
  (if (`self.CanGivePoint`)
    (set `self.CanGivePoint` false)
    (`/Game/Cats/Blueprint/MainLibrary.AddBadKarma` 25)
    (`NiagaraFunctionLibrary.SpawnSystemAtLocation` "/Game/Cats/Assets/Points/bad_25_FX_System.bad_25_FX_System" (+ Localisation (0.0 0.0 50.0)) (struct) (0.8 0.8 0.8))))

(fn `UserConstructionScript`)