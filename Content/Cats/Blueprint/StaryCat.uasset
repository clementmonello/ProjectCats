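; StaryCat is a cat Blueprint that moves with a floating pawn movement component and a spline-following component.
; SetSpeed keeps the follow-spline speed and the movement component's max speed in sync.
; SetDefaulltValue configures the cat through SetSpeed and passes the forward aim distance and debug-draw setting to the spline follower.
; The event graph holds only disabled stubs, so this Blueprint's own graphs only provide configuration.
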(fn `setDefaulltValue`
  (params (Speed :type "Float (double-precision)") (ForwardAimDistance :type "Float (double-precision)") (DrawDebugAimDistance :type Boolean))
  (bind _bp_followsplinecomponent (`self.BP_FollowSplineComponent`))
  (`self.SetSpeed` Speed)
  (set `/Game/Cats/Blueprint/Component/C_FollowSplineComponent.ForwardAimDistance` ForwardAimDistance _bp_followsplinecomponent)
  (set `/Game/Cats/Blueprint/Component/C_FollowSplineComponent.DrawDebug` DrawDebugAimDistance _bp_followsplinecomponent))

(fn `SetSpeed`
  (params (NewSpeed :type "Float (double-precision)"))
  (set `/Game/Cats/Blueprint/Component/C_FollowSplineComponent.Speed` NewSpeed (`self.BP_FollowSplineComponent`))
  (set `FloatingPawnMovement.MaxSpeed` NewSpeed (`self.FloatingPawnMovement`)))

(fn `UserConstructionScript`
  (`parent.UserConstructionScript`))