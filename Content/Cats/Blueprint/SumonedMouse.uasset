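; Summoned winged AI mouse that hunts a Damageable actor and dies in an explosion when it hits it or its lifetime runs out.
; Perception claims a target no other summoned mouse holds and writes it to the Blackboard, while Tick drains the life bar.
; Hitting the target sends it a damage message; taking damage kills the mouse and awards nice karma.
; Die flags the Blackboard, stops movement and Tick, enables mesh physics and spawns the chosen Niagara effect.
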(event `self.ReceiveAnyDamage`
  (params (Damage :type "Float (single-precision)") (DamageType :type "DamageType Object Reference") (InstigatedBy :type "Controller Object Reference") (DamageCauser :type "Actor Object Reference"))
  (`self.Attacked`))

(event `self.ReceiveActorBeginOverlap`
  (params (OtherActor :type "Actor Object Reference"))
  (`parent.ReceiveActorBeginOverlap` OtherActor))

(event `self.ReceiveTick`
  (params (DeltaSeconds :type "Float (single-precision)"))
  (`parent.ReceiveTick` DeltaSeconds)
  (if (<= (`self.TimeRemaining`) 0.0)
    (set `self.NiagaraSystem` "/Niagara/DefaultAssets/Templates/Systems/SimpleExplosion.SimpleExplosion")
    (`self.Die`)
    (else
      (bind _output_get (set `self.TimeRemaining` (- (`self.TimeRemaining`) DeltaSeconds)))
      (`/Game/Cats/Widget/MouseLifeBar.SetProgressBar` (`self.As Mouse Life Bar`) (`KismetMathLibrary.FClamp` (/ _output_get (`self.LifeTime`)))))))

(event `self.ReceiveBeginPlay`
  (`parent.ReceiveBeginPlay`)
  (set `self.NiceKarmaPoint` 25)
  (set `self.TimeRemaining` (`self.LifeTime`))
  (bind _asmouse_life_bar (cast `/Game/Cats/Widget/MouseLifeBar` (`WidgetComponent.GetWidget` (`self.LifeBar`))))
  (set `self.As Mouse Life Bar` _asmouse_life_bar))

(event `self.AIPerception.OnTargetPerceptionUpdated`
  (params (Actor :type "Actor Object Reference") (Stimulus :type "AIStimulus Structure"))
  (if (not (`KismetSystemLibrary.IsValid` (`self.Target`)))
    (set `self.targettaken` false)
    (if (`KismetSystemLibrary.DoesImplementInterface` Actor "/Game/Cats/Blueprint/Interfaces/damageable.damageable_C")
      (bind _outactors (`GameplayStatics.GetAllActorsOfClass` "SumonedMouse_C"))
      (for _array_element _outactors
        (bind _target (`/Game/Cats/Blueprint/SumonedMouse.Target` _array_element))
        (if (`KismetSystemLibrary.IsValid` _target)
          (if (== _target Actor)
            (set `self.targettaken` true))))
      (if (not (`self.targettaken`))
        (set `self.Target` Actor)
        (`BlackboardComponent.SetValueAsObject` (`AIBlueprintHelperLibrary.GetBlackboard` (`self.GetController` self)) (`self.TargetName`) Actor)))))

(event `self.ReceiveHit`
  (params (MyComp :type "PrimitiveComponent Object Reference") (Other :type "Actor Object Reference") (OtherComp :type "PrimitiveComponent Object Reference") (bSelfMoved :type Boolean) (HitLocation :type "Vector Structure") (HitNormal :type "Vector Structure") (NormalImpulse :type "Vector Structure") (Hit :type "HitResult Structure (by ref)"))
  (bind _target (`self.Target`))
  (if (== Other _target)
    (set `self.NiagaraSystem` "/Niagara/DefaultAssets/Templates/Systems/SimpleExplosion.SimpleExplosion")
    (`self.Die`)
    (message `/Game/Cats/Blueprint/Interfaces/damageable.On Damage` _target (`self.K2_GetActorLocation` _target))))

(fn `Attacked`
  (`/Game/Cats/Blueprint/MainLibrary.AddNiceKarma` (`self.NiceKarmaPoint`))
  (set `self.NiagaraSystem` "/Game/Cats/Assets/Points/nice_25_fx_System.nice_25_fx_System")
  (`self.Die`))

(fn `Die`
  (bind _returnvalue (`self.GetController` self))
  (`PrimitiveComponent.SetSimulatePhysics` (`self.SkeletalMesh`) true)
  (`BlackboardComponent.SetValueAsBool` (`AIBlueprintHelperLibrary.GetBlackboard` _returnvalue) "Dead" true)
  (if (not (`self.Dead`))
    (`SceneComponent.K2_AddLocalRotation` (`self.DefaultSceneRoot`) (struct :`Roll` 90.0) false false)
    (set `self.Dead` true)
    (`Controller.StopMovement` _returnvalue)
    (`NiagaraFunctionLibrary.SpawnSystemAtLocation` (`self.NiagaraSystem`) (`self.K2_GetActorLocation`))
    (`SkeletalMeshComponent.Stop` (`self.SkeletalMesh`))
    (`SkeletalMeshComponent.Stop` (`self.Wings`))
    (`SkeletalMeshComponent.Stop` (`self.Wings1`))
    (`SceneComponent.SetVisibility` (`self.LifeBar`) false true)
    (`self.SetActorTickEnabled` false)))

(fn `PickLocation`
  (returns (Location :type "Vector Structure"))
  (locals (PickedPoint :type "Vector Structure"))
  (return (`NavigationSystemV1.K2_GetRandomReachablePointInRadius` (`self.K2_GetActorLocation`) 800.0 null null)))

(fn `StopBlackboard`
  (`BrainComponent.StopLogic` (`AIController.BrainComponent` (`AIBlueprintHelperLibrary.GetAIController` self)) ""))

(fn `UserConstructionScript`
  (`parent.UserConstructionScript`))