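; MainLibrary is a Blueprint function library for adding karma to the player's cat.
; AddNiceKarma and AddBadKarma each cast player character 0 to Cat and add the given points to its NiceKarma or BadKarma variable.
; Both functions do nothing if that character is not a Cat.
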(fn `AddBadKarma`
  (params (Points :type Integer))
  (bind _ascat (cast `/Game/Cats/Blueprint/Cat` (`GameplayStatics.GetPlayerCharacter` (`local.__WorldContext`))))
  (set `/Game/Cats/Blueprint/Cat.BadKarma` (+ Points (`/Game/Cats/Blueprint/Cat.BadKarma` _ascat)) _ascat))

(fn `AddNiceKarma`
  (params (points :type Integer))
  (bind _ascat (cast `/Game/Cats/Blueprint/Cat` (`GameplayStatics.GetPlayerCharacter` (`local.__WorldContext`))))
  (set `/Game/Cats/Blueprint/Cat.NiceKarma` (+ points (`/Game/Cats/Blueprint/Cat.NiceKarma` _ascat)) _ascat))