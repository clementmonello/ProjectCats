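; Mouse NPC, prey that dies when a Cat overlaps it.
; Attacked turns on mesh physics, sets Dead on itself and its blackboard, stops movement and decrements its MouseArea's live count.
; PickLocation retries random points in the area's spline bounds until a ray-casting test puts one inside its polygon, falling back to a nearby reachable point without an area.
; MoveNPC is outdated and unused, replaced by a behavior tree.
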(event `self.ReceiveActorBeginOverlap`
  (params (OtherActor :type "Actor Object Reference"))
  (`parent.ReceiveActorBeginOverlap` OtherActor)
  (cast `/Game/Cats/Blueprint/Cat` OtherActor)
  (`self.Attacked`))

(event `self.ReceiveBeginPlay`
  (`parent.ReceiveBeginPlay`)
  (set `self.BadKarmaPoint` 100))

(event `MoveNPC`
  ;[1 1 1] OutDated - c'est le behaviour tree mtn
  (bind _location (`self.PickLocation`))
  (bind _output_get (set `self.RandomLocation` _location))
  (`|AIMoveTo` self _output_get null
    (:`OnSuccess`
      _)
    (:`OnFail`
      _))
  (`KismetSystemLibrary.Delay` (`KismetMathLibrary.RandomFloatInRange` 0.0 2.0))
  (if (`self.Dead`)
    _))

(fn `Attacked`
  (bind _mousearea (`self.MouseArea`))
  (bind _returnvalue (`self.GetController` self))
  (`PrimitiveComponent.SetSimulatePhysics` (`self.SkeletalMesh`) true)
  (`BlackboardComponent.SetValueAsBool` (`AIBlueprintHelperLibrary.GetBlackboard` _returnvalue) "Dead" true)
  (set `self.Dead` true)
  (`Controller.StopMovement` _returnvalue)
  (if (`KismetSystemLibrary.IsValid` _mousearea)
    (`/Game/Cats/Blueprint/MouseArea.DecreaseMouseAlive` _mousearea)))

(fn `IsPointInPolygon`
  (params (Point :type "Vector Structure") (Polygon :type "Array of Vector Structure"))
  (returns (isInside :type Boolean))
  (locals (NumPoints :type Integer) (Return :type Boolean) (indexi :type Integer) (indexj :type Integer))
  (bind _numpoints (`local.NumPoints`))
  (bind (_point_x _point_y) (`KismetMathLibrary.BreakVector` (`local.Point`)))
  (bind (_point_x_2 _point_y_2) (`KismetMathLibrary.BreakVector` (`local.Point`)))
  (bind (_point_x_3 _point_y_3) (`KismetMathLibrary.BreakVector` (`local.Point`)))
  (bind (_output_x _output_y) (`KismetMathLibrary.BreakVector` (`|GetArrayItem` (`local.Polygon`) (`local.indexi`))))
  (bind _output_x_2 (`KismetMathLibrary.BreakVector` (`|GetArrayItem` (`local.Polygon`) (`local.indexi`))))
  (bind (_output_x_3 _output_y_2) (`KismetMathLibrary.BreakVector` (`|GetArrayItem` (`local.Polygon`) (`local.indexi`))))
  (bind (_output_x_4 _output_y_3) (`KismetMathLibrary.BreakVector` (`|GetArrayItem` (`local.Polygon`) (`local.indexj`))))
  (bind (_output_x_5 _output_y_4) (`KismetMathLibrary.BreakVector` (`|GetArrayItem` (`local.Polygon`) (`local.indexj`))))
  (bind _output_x_6 (`KismetMathLibrary.BreakVector` (`|GetArrayItem` (`local.Polygon`) (`local.indexj`))))
  (set `local.NumPoints` (`KismetArrayLibrary.Array_Length` Polygon))
  (set `local.Return` false)
  (for _index (range (`local.NumPoints`))
    (bind _output_get (set `local.indexi` _index))
    (set `local.indexj` (mod (+ _output_get _numpoints -1) _numpoints))
    (if (and (!= (> _output_y_2 _point_y_3) (> _output_y_3 _point_y)) (< _point_x_2 (+ (* (- _output_x_6 _output_x_2) (/ (- _point_y_2 _output_y) (- _output_y_4 _output_y))) _output_x)))
      (set `local.Return` (not (`local.Return`)))))
  (return (`local.Return`)))

(fn `PickLocation`
  (returns (Location :type "Vector Structure"))
  (locals (PickedPoint :type "Vector Structure"))
  (bind (_origin _boxextent) (`KismetSystemLibrary.GetComponentBounds` (`/Game/Cats/Blueprint/MouseArea.Spline` (`self.MouseArea`))))
  (if (`KismetSystemLibrary.IsValid` (`self.MouseArea`))
    (bind _output_get (set `local.PickedPoint` (`KismetMathLibrary.RandomPointInBoundingBox` _origin _boxextent) :!label _label))
    (bind _isinside (`self.IsPointInPolygon` _output_get (`/Game/Cats/Blueprint/MouseArea.Polygon` (`self.MouseArea`))))
    (if _isinside
      (return (`local.PickedPoint`))
      (else
        (goto _label)))
    (else
      (return (`NavigationSystemV1.K2_GetRandomReachablePointInRadius` (`self.K2_GetActorLocation`) 200.0 null null)))))

(fn `StopBlackboard`
  (`BrainComponent.StopLogic` (`AIController.BrainComponent` (`AIBlueprintHelperLibrary.GetAIController` self)) ""))

(fn `UserConstructionScript`
  (`parent.UserConstructionScript`))