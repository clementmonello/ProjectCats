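; DogsChasing is a spline-following dog pawn for a chase quest that players can damage and take out.
; A setup function receives speed, HP, quest reference and aim distance, driving both the follow-spline component and floating movement.
; Each hit lowers HP and tells the quest to increase speed.
; At zero HP it reports the kill, spawns a Niagara karma effect and hides the actor rather than destroying it.
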(event `self.ReceiveBeginPlay`
  (`parent.ReceiveBeginPlay`)
  (set `self.NiceKarmaPoint` 200)
  (set `self.NiagaraSystem` "/Niagara/DefaultAssets/Templates/Systems/DirectionalBurst.DirectionalBurst"))

(event `/Game/Cats/Blueprint/Interfaces/damageable.On Damage`
  (params (Localisation :type "Vector Structure"))
  (bind _quest (`self.Quest`))
  (set `self.HP` (- (`self.HP`) 1))
  (`/Game/Cats/Blueprint/QuestDogChase.IncreaseSpeed` _quest)
  (if (<= (`self.HP`) 0)
    (`/Game/Cats/Blueprint/QuestDogChase.DogKill` _quest)
    (`NiagaraFunctionLibrary.SpawnSystemAtLocation` "/Game/Cats/Assets/Points/nice_200_FX_System.nice_200_FX_System" Localisation)
    (`self.SetActorHiddenInGame` self true)))

(fn `Set Defaullt Value`
  (params (Speed :type "Float (double-precision)") (ForwardAimDistance :type "Float (double-precision)") (HP :type Integer) (Quest :type "/Game/Cats/Blueprint/QuestDogChase Object Reference") (DrawDebugAimDistance :type Boolean))
  (bind _bp_followsplinecomponent (`self.BP_FollowSplineComponent`))
  (`self.SetSpeed` Speed)
  (set `self.Quest` Quest)
  (set `self.HP` HP)
  (set `/Game/Cats/Blueprint/Component/BP_FollowSplineComponent.ForwardAimDistance` ForwardAimDistance _bp_followsplinecomponent)
  (set `/Game/Cats/Blueprint/Component/BP_FollowSplineComponent.DrawDebug` DrawDebugAimDistance _bp_followsplinecomponent))

(fn `SetSpeed`
  (params (NewSpeed :type "Float (double-precision)"))
  (set `/Game/Cats/Blueprint/Component/BP_FollowSplineComponent.Speed` NewSpeed (`self.BP_FollowSplineComponent`))
  (set `FloatingPawnMovement.MaxSpeed` NewSpeed (`self.FloatingPawnMovement`)))

(fn `UserConstructionScript`
  (`parent.UserConstructionScript`))