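; Juggler mission actor where the cat brings balls, ending in 500 nice or bad karma based on the paper ball count.
; A looping timeline moves collected, randomly spinning balls along a spline, offset evenly by index.
; BeginPlay scatters balls and paper balls at random line-traced points nearby.
; An overlap area toggles the mission widget; AddBall resolves the mission once the total is reached.
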(event `self.ReceiveTick`
  (params (DeltaSeconds :type "Float (single-precision)"))
  (for _array_element (`self.Balls`)
    (`SceneComponent.K2_AddLocalRotation` _array_element (`KismetMathLibrary.MakeRotator` (`KismetMathLibrary.RandomFloatInRange` 0.0 8.0) (`KismetMathLibrary.RandomFloatInRange` 0.0 8.0) (`KismetMathLibrary.RandomFloatInRange` 0.0 8.0)) false false)))

(event `self.ReceiveBeginPlay`
  (bind _balls (`self.Balls`))
  (`KismetArrayLibrary.Array_Add` _balls (`self.Sphere`))
  (`KismetArrayLibrary.Array_Add` _balls (`self.Sphere1`))
  (`TimelineComponent.SetPlayRate` (`self.PositionAlpha`) 0.5)
  (`self.Play Timeline`)
  (bind _output_get (set `self.whileIndex` 0))
  (while (> (`self.PaperBallCount`) _output_get)
    (`self.spawnPaper`)
    (`/Engine/EditorBlueprintResources/StandardMacros.IncrementInt` _output_get))
  (bind _output_get_2 (set `self.whileIndex` 0))
  (while (> (`self.BallCount`) _output_get_2)
    (`self.spawnBall`)
    (`/Engine/EditorBlueprintResources/StandardMacros.IncrementInt` _output_get_2)))

(event `Play Timeline`
  (bind _spline (`self.Spline`))
  (bind _returnvalue (`SplineComponent.GetDistanceAlongSplineAtSplinePoint` _spline (`SplineComponent.GetNumberOfSplinePoints` _spline)))
  (bind (_direction _alpha) (`Timeline|PositionAlpha` :!via `PlayFromStart`)
    (:`Update`
      (for (_array_element _array_index) (`self.Balls`)
        (`SceneComponent.K2_SetWorldLocation` _array_element (`SplineComponent.GetLocationAtDistanceAlongSpline` (`self.Spline`) (mod (`KismetMathLibrary.Lerp` 0.0 _returnvalue (+ _alpha (* (`KismetMathLibrary.Conv_IntToDouble` _array_index) (/ 1.0 (`KismetMathLibrary.Conv_IntToDouble` (`KismetArrayLibrary.Array_Length` (`self.Balls`))))))) _returnvalue) "World") false false)))
    (:`Finished`
      (`self.Play Timeline`))))

(event `GoodOrBad`
  (params (isBad :type Boolean))
  (bind _widgetmission (`self.WidgetMission`))
  (set `self.CanGetBalls` false)
  (bind _output_get (set `self.bad` isBad))
  (if _output_get
    (`/Game/Cats/Blueprint/MainLibrary.AddBadKarma` 500)
    (else
      (`/Game/Cats/Blueprint/MainLibrary.AddNiceKarma` 500)))
  (`NiagaraFunctionLibrary.SpawnSystemAtLocation` (select `bool` _output_get :`false` "/Game/Cats/Assets/Points/nice_500_FX_System.nice_500_FX_System" :`true` "/Game/Cats/Assets/Points/bad_500_FX_System.bad_500_FX_System" :!type "NiagaraSystem Object Reference") (+ (`self.K2_GetActorLocation`) (0.0 0.0 10.0)))
  (set `self.MissionDone` true)
  (`/Engine/EditorBlueprintResources/StandardMacros.IsValid` (`self.WidgetMission`) :!label _label
    (:`Is Valid`
      (`UserWidget.PlayAnimation` _widgetmission (`/Game/Cats/Widget/GoodMissionMenu.NewMission` _widgetmission) 0.0 1 "Reverse" 1.0 false)
      (`KismetSystemLibrary.Delay` 0.3)
      (`Widget.RemoveFromParent` _widgetmission))))

(event `self.Entering Area.OnComponentEndOverlap`
  (params (OverlappedComponent :type "PrimitiveComponent Object Reference") (OtherActor :type "Actor Object Reference") (OtherComp :type "PrimitiveComponent Object Reference") (OtherBodyIndex :type Integer))
  (if (not (`self.MissionDone`))
    (cast `/Game/Cats/Blueprint/Cat` OtherActor)
    (goto _label)))

(event `self.Entering Area.OnComponentBeginOverlap`
  (params (OverlappedComponent :type "PrimitiveComponent Object Reference") (OtherActor :type "Actor Object Reference") (OtherComp :type "PrimitiveComponent Object Reference") (OtherBodyIndex :type Integer) (bFromSweep :type Boolean) (SweepResult :type "HitResult Structure (by ref)"))
  (if (not (`self.MissionDone`))
    (cast `/Game/Cats/Blueprint/Cat` OtherActor)
    (bind _returnvalue (`|CreateWidget` "/Game/Cats/Widget/GoodMissionMenu.GoodMissionMenu_C" (`GameplayStatics.GetPlayerController` 0)))
    (set `/Game/Cats/Widget/GoodMissionMenu.GoodMissionText` "Bring balls to Juggler" _returnvalue)
    (bind _output_get (set `self.WidgetMission` _returnvalue))
    (`UserWidget.AddToViewport` _output_get 0)
    (`UserWidget.PlayAnimation` _output_get (`/Game/Cats/Widget/GoodMissionMenu.NewMission` _output_get) 0.1 1 "Forward" 1.0 false)))

(fn `addBall`
  (params (BallMesh :type "StaticMeshComponent Object Reference (by ref)"))
  (if (`self.CanGetBalls`)
    (`PrimitiveComponent.SetCollisionResponseToChannel` BallMesh "ECC_Camera" "ECR_Ignore")
    (bind _returnvalue (`KismetArrayLibrary.Array_Add` (`self.Balls`) BallMesh))
    (if (>= _returnvalue (- (`self.TotalBall`) 1))
      (`self.GoodOrBad` (> (`self.BadCount`) (`self.PaperBallAllowed`))))))

(fn `getSpawnPoint`
  (returns (`Out Hit Location` :type "Vector Structure"))
  (bind _sizespawn (`self.SizeSpawn`))
  (bind _returnvalue (`KismetMathLibrary.RandomPointInBoundingBox` (+ (`self.K2_GetActorLocation`) (`KismetMathLibrary.MakeVector` 0.0 0.0 (`self.SizeSpawn`))) (`KismetMathLibrary.MakeVector` _sizespawn _sizespawn _sizespawn)))
  (bind _outhit (`KismetSystemLibrary.LineTraceSingle` _returnvalue (- _returnvalue (`KismetMathLibrary.MakeVector` 0.0 0.0 (* (`self.SizeSpawn`) 5.0))) "TraceTypeQuery1"))
  (return (`.Location` (`GameplayStatics.BreakHitResult` _outhit))))

(fn `spawnBall`
  (bind _out_hit_location (`self.getSpawnPoint`))
  (`|SpawnActorFromClass` "/Game/Cats/Blueprint/Balls.Balls_C" (`KismetMathLibrary.MakeTransform` _out_hit_location (`KismetMathLibrary.RandomRotator` false)) "AdjustIfPossibleButAlwaysSpawn" "MultiplyWithRoot" null null))

(fn `spawnPaper`
  (bind _out_hit_location (`self.getSpawnPoint`))
  (`|SpawnActorFromClass` "/Game/Cats/Blueprint/PaperBall.PaperBall_C" (`KismetMathLibrary.MakeTransform` _out_hit_location (`KismetMathLibrary.RandomRotator` false)) "AdjustIfPossibleButAlwaysSpawn" "MultiplyWithRoot" null null))

(fn `UserConstructionScript`)