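; MissionArea is a placed trigger actor that shows a mission prompt to the player's Cat.
; When a Cat enters the Activate volume, it creates a GoodMissionMenu widget with the area's MissionText and plays its NewMission animation.
; When a Cat leaves the Desactivate volume, it plays that animation in reverse, then removes the widget after a short delay.
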(event `self.Activate.OnComponentBeginOverlap`
  (params (OverlappedComponent :type "PrimitiveComponent Object Reference") (OtherActor :type "Actor Object Reference") (OtherComp :type "PrimitiveComponent Object Reference") (OtherBodyIndex :type Integer) (bFromSweep :type Boolean) (SweepResult :type "HitResult Structure (by ref)"))
  (cast `/Game/Cats/Blueprint/Cat` OtherActor)
  (bind _returnvalue (`|CreateWidget` "/Game/Cats/Widget/GoodMissionMenu.GoodMissionMenu_C" (`GameplayStatics.GetPlayerController` 0)))
  (set `/Game/Cats/Widget/GoodMissionMenu.GoodMissionText` (`self.MissionText`) _returnvalue)
  (bind _output_get (set `self.WidgetMission` _returnvalue))
  (`UserWidget.AddToViewport` _output_get 0)
  (`UserWidget.PlayAnimation` _output_get (`/Game/Cats/Widget/GoodMissionMenu.NewMission` _output_get) 0.1 1 "Forward" 1.0 false))

(event `self.Desactivate.OnComponentEndOverlap`
  (params (OverlappedComponent :type "PrimitiveComponent Object Reference") (OtherActor :type "Actor Object Reference") (OtherComp :type "PrimitiveComponent Object Reference") (OtherBodyIndex :type Integer))
  (bind _widgetmission (`self.WidgetMission`))
  (`/Engine/EditorBlueprintResources/StandardMacros.IsValid` (`self.WidgetMission`)
    (:`Is Valid`
      (cast `/Game/Cats/Blueprint/Cat` OtherActor)
      (`UserWidget.PlayAnimation` _widgetmission (`/Game/Cats/Widget/GoodMissionMenu.NewMission` _widgetmission) 0.0 1 "Reverse" 1.0 false)
      (`KismetSystemLibrary.Delay` 0.3)
      (`Widget.RemoveFromParent` _widgetmission))))

(fn `UserConstructionScript`)