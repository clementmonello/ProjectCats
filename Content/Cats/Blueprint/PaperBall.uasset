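; PaperBall is a pickup actor that a Jongleur character collects as a crumpled paper ball to juggle, counted as a bad catch.
; When its Sphere overlaps the Jongleur's capsule and CanGetBalls is true, it adds a small crumpled-paper static mesh component to the Jongleur.
; It passes that mesh to AddBall, increments BadCount, then destroys itself.
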(event `self.Sphere.OnComponentBeginOverlap`
  (params (OverlappedComponent :type "PrimitiveComponent Object Reference") (OtherActor :type "Actor Object Reference") (OtherComp :type "PrimitiveComponent Object Reference") (OtherBodyIndex :type Integer) (bFromSweep :type Boolean) (SweepResult :type "HitResult Structure (by ref)"))
  (bind _asjongleur (cast `/Game/Cats/Blueprint/Jongleur` OtherActor))
  (cast `CapsuleComponent` OtherComp)
  (if (`/Game/Cats/Blueprint/Jongleur.CanGetBalls` _asjongleur)
    (bind _returnvalue (`AddComponent|NODE_AddStaticMeshComponent-0` :`self` _asjongleur :`RelativeTransform` (`KismetMathLibrary.MakeTransform` (0.0 0.0 0.0) (struct) (0.1 0.1 0.1))))
    (`StaticMeshComponent.SetStaticMesh` _returnvalue "/Game/Cats/Assets/Props/crumpled_paper.crumpled_paper")
    (`/Game/Cats/Blueprint/Jongleur.addBall` _asjongleur _returnvalue)
    (bind _result (`/Engine/EditorBlueprintResources/StandardMacros.IncrementInt` (`/Game/Cats/Blueprint/Jongleur.BadCount` _asjongleur))
      (:`  `
        (set `/Game/Cats/Blueprint/Jongleur.BadCount` _result _asjongleur)
        (`self.K2_DestroyActor`)))))

(fn `UserConstructionScript`)