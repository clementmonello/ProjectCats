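; Adult NPC that wanders the level until a Cat overlaps it and kills it.
; On overlap its mesh switches to physics simulation, it is flagged dead and its controller stops moving.
; Wandering loops from BeginPlay: a random delay, then an AI move to a random reachable nearby point, repeating on success or failure while alive.
; It also sets its bad karma point value at start.
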(event `self.ReceiveActorBeginOverlap`
  (params (OtherActor :type "Actor Object Reference"))
  (`parent.ReceiveActorBeginOverlap` OtherActor)
  (cast `/Game/Cats/Blueprint/Cat` OtherActor)
  (`PrimitiveComponent.SetSimulatePhysics` (`self.SkeletalMesh`) true)
  (set `self.Dead` true)
  (`Controller.StopMovement` (`self.GetController` self)))

(event `self.ReceiveTick`
  (params (DeltaSeconds :type "Float (single-precision)"))
  (`parent.ReceiveTick` DeltaSeconds))

(event `self.ReceiveBeginPlay`
  (`parent.ReceiveBeginPlay`)
  (set `self.BadKarmaPoint` 50)
  (`KismetSystemLibrary.Delay` (`KismetMathLibrary.RandomFloatInRange` 2.0 10.0) :!label _label)
  (if (not (`self.Dead`))
    (`self.MoveNPC`)))

(event `MoveNPC`
  (bind _output_get (set `self.RandomLocation` (`NavigationSystemV1.K2_GetRandomReachablePointInRadius` (`self.K2_GetActorLocation`) 1000.0 null null)))
  (`|AIMoveTo` self _output_get null
    (:`OnSuccess`
      (goto _label))
    (:`OnFail`
      (goto _label))))

(fn `UserConstructionScript`
  (`parent.UserConstructionScript`))