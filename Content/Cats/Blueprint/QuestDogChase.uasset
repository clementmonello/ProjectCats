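; Quest actor for a dog chase, in which a dog pursues a stray cat with spline-following movement.
; On BeginPlay it configures the assigned pair, or spawns defaults at the path start with the dog behind, creating a looped fallback spline if none is set.
; The dog receives HP and a quest reference; DogKill flags its death and stops both movers.
; IncreaseSpeed raises both max speeds by ten percent.
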(event `self.ReceiveBeginPlay`
  (bind _speed (`self.Speed`))
  (bind _forwardaimdistance (`self.ForwardAimDistance`))
  (if (not (`KismetSystemLibrary.IsValid` (`self.Path`)))
    (`KismetSystemLibrary.PrintString` "No path provided for dog chase" true true (struct :`R` 1.0 :`B` 0.015037 :`A` 1.0) 10.0 "NoPath")
    (`self.MakeDefaultPath`))
  (if (not (and (`KismetSystemLibrary.IsValid` (`self.Stary`)) (`KismetSystemLibrary.IsValid` (`self.Dog`))))
    (`self.SpawnActors`)
    (`KismetSystemLibrary.PrintString` "No Cats and Dogs were specified. The default ones are used instead" true true (struct :`R` 1.0 :`B` 0.059916 :`A` 1.0) 20.0)
    (else
      (`/Game/Cats/Blueprint/DogsChasing.setDefaulltValue` (`self.Dog`) _speed _forwardaimdistance (`self.DogHP`) self)
      (`/Game/Cats/Blueprint/StaryCat.setDefaulltValue` (`self.Stary`) _speed _forwardaimdistance))))

(fn `DogKill`
  (set `self.DogIsKilled` true)
  (`ActorComponent.Deactivate` (`/Game/Cats/Blueprint/BaseEntity.FloatingPawnMovement` (`self.Stary`)))
  (`ActorComponent.Deactivate` (`/Game/Cats/Blueprint/BaseEntity.FloatingPawnMovement` (`self.Dog`))))

(fn `IncreaseSpeed`
  (bind _returnvalue (`self.GetComponentByClass` (`self.Dog`) "/Script/Engine.FloatingPawnMovement"))
  (bind _returnvalue_2 (`self.GetComponentByClass` (`self.Stary`) "/Script/Engine.FloatingPawnMovement"))
  (set `FloatingPawnMovement.MaxSpeed` (* (`FloatingPawnMovement.MaxSpeed` _returnvalue_2) 1.1) _returnvalue_2)
  (set `FloatingPawnMovement.MaxSpeed` (* (`FloatingPawnMovement.MaxSpeed` _returnvalue) 1.1) _returnvalue))

(fn `MakeDefaultPath`
  (bind _returnvalue (`|SpawnActorFromClass` "/Game/Cats/Blueprint/BP_TargetSpline.BP_TargetSpline_C" (`self.GetTransform`) "AlwaysSpawn" "MultiplyWithRoot" null null))
  (bind _output_get (set `self.Path` _returnvalue))
  (bind _spline (`/Game/Cats/Blueprint/BP_TargetSpline.Spline` _output_get))
  (`SplineComponent.AddSplinePoint` _spline (`KismetMathLibrary.MakeVector` 500.0) "Local" true)
  (`SplineComponent.AddSplinePoint` _spline (`KismetMathLibrary.MakeVector` 500.0 500.0) "Local" true)
  (`SplineComponent.SetClosedLoop` _spline true true))

(fn `SpawnActors`
  (bind _stary (`self.Stary`))
  (bind _returnvalue (`self.K2_GetActorLocation` _stary))
  (bind _returnvalue_2 (`SplineComponent.GetTransformAtSplinePoint` (`/Game/Cats/Blueprint/BP_TargetSpline.Spline` (`self.Path`)) 0 "World" false))
  (bind (_returnvalue_x _returnvalue_y) (`KismetMathLibrary.BreakVector` (- _returnvalue (* (`self.GetActorForwardVector` _stary) 200.0))))
  (bind _returnvalue_3 (`|SpawnActorFromClass` "/Game/Cats/Blueprint/StaryCat.StaryCat_C" _returnvalue_2 "AdjustIfPossibleButAlwaysSpawn" "MultiplyWithRoot" null null))
  (bind _output_get (set `self.Stary` _returnvalue_3))
  (set `/Game/Cats/Blueprint/Component/BP_FollowSplineComponent.ForwardAimDistance` 100.0 (`/Game/Cats/Blueprint/StaryCat.BP_FollowSplineComponent` _output_get))
  (`/Game/Cats/Blueprint/StaryCat.SetSpeed` _output_get (`self.Speed`))
  (bind _returnvalue_4 (`|SpawnActorFromClass` "/Game/Cats/Blueprint/DogsChasing.DogsChasing_C" (`KismetMathLibrary.MakeTransform` (`KismetMathLibrary.MakeVector` _returnvalue_x _returnvalue_y (.z _returnvalue)) (.rotation _returnvalue_2)) "AdjustIfPossibleButAlwaysSpawn" "MultiplyWithRoot" null null))
  (bind _output_get_2 (set `self.Dog` _returnvalue_4))
  (set `/Game/Cats/Blueprint/DogsChasing.Quest` self _output_get_2)
  (set `/Game/Cats/Blueprint/DogsChasing.HP` (`self.DogHP`) _output_get_2)
  (`/Game/Cats/Blueprint/DogsChasing.SetSpeed` _output_get_2 (`self.Speed`))
  (set `/Game/Cats/Blueprint/Component/BP_FollowSplineComponent.ForwardAimDistance` 100.0 (`/Game/Cats/Blueprint/DogsChasing.BP_FollowSplineComponent` _output_get_2)))

(fn `UserConstructionScript`)